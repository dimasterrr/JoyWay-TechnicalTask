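; Player character pawn that sets up the player HUD on possession and requests its own respawn when destroyed.
; After a short delay on possession, it shows the player screen widget through the base player HUD and sets an unpaused, non-UI-only HUD mode focused on that widget.
; On destruction, it runs the parent logic, then passes itself to BP_GameMode's respawn function.
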(event EventPossessed
  (params (NewController :type Controller%20Object%20Reference))
  (Utilities|FlowControl|Delay 0.2)
  (bind _returnvalue (Class|PlayerHudBase|ShowWidget (Class|GeneralHelper|GetBasePlayerHud) "PlayerScreen"))
  (Class|PlayerHudBase|SetHudMode (Class|GeneralHelper|GetBasePlayerHud) false false _returnvalue))

(event EventDestroyed
  (|CallParentFunction)
  (bind _asbp_game_mode (Utilities|Casting|CastToBP_GameMode (Game|GetGameMode)))
  (Default|ReSpawnPlayer _asbp_game_mode self))

(fn ConstructionScript)